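; Box spawner actor that spawns Box actors at its own transform at an accelerating rate, starting on BeginPlay.
; SpawnBox spawns even when colliding, increments BoxCount, then re-arms itself with a timer by function name.
; Each call shrinks SpawnDelay geometrically until it reaches a small floor, and spawning continues with no count limit.
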(event EventBeginPlay
  (Utilities|Time|SetTimerbyFunctionName 0 "SpawnBox" (Variables|Default|GetSpawnDelay))
  (CallFunction|SpawnBox))

(fn ConstructionScript)

(fn SpawnBox
  (Game|SpawnActorfromClass "/Game/Blueprints/Box.Box_C" (Transformation|GetActorTransform) true 0)
  (Variables|Default|SetBoxCount (+ (Variables|Default|GetBoxCount) 1))
  (if (> (Variables|Default|GetSpawnDelay) 0.01)
    (Variables|Default|SetSpawnDelay (* (Variables|Default|GetSpawnDelay) 0.9)))
  (Utilities|Time|SetTimerbyFunctionName 0 "SpawnBox" (Variables|Default|GetSpawnDelay)))