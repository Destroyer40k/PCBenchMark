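; MetricManager records frame-rate metrics over a play session and saves them as a DemoResults save game.
; Tick counts total and per-second frames, using game time to close each roughly one-second window and update minimum and maximum FPS.
; Window updates are held back until over a second after BeginPlay.
; EndPlay writes both extremes, the frame count and the session duration to the DataSlotName slot.
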(event EventTick
  (params (DeltaSeconds :type Float%20%28single-precision%29))
  (Variables|Default|SetCurrentSecondFrames (+ (Variables|Default|GetCurrentSecondFrames) 1))
  (Variables|Default|SetFrameCount (+ (Variables|Default|GetFrameCount) 1))
  (bind _isdifferentsecond (CallFunction|DifferentSecond))
  (if (Math|Boolean|Equal(Boolean) _isdifferentsecond true)
    (CallFunction|ChangeSecond)))

(event EventBeginPlay
  (Variables|Default|SetBeginTime (Utilities|Time|GetGameTimeinSeconds)))

(event EventEndPlay
  (params (EndPlayReason :type EEndPlayReason%20Enum :default "ActorDestroyed"))
  (Variables|Default|SetEndTime (Utilities|Time|GetGameTimeinSeconds))
  (bind _returnvalue (SaveGame|CreateSaveGameObject "/Game/Blueprints/DataContainerObjects/DemoResults.DemoResults_C"))
  (bind _asdemoresults_c (Utilities|Casting|CastToDemoResults _returnvalue))
  (Variables|/Game/Blueprints/DataContainerObjects/DemoResults.DemoResults_C|SetMinFPS _asdemoresults_c (Variables|Default|GetMinFPS))
  (Variables|/Game/Blueprints/DataContainerObjects/DemoResults.DemoResults_C|SetFrameCount _asdemoresults_c (Variables|Default|GetFrameCount))
  (Variables|/Game/Blueprints/DataContainerObjects/DemoResults.DemoResults_C|SetMaxFPS _asdemoresults_c (Variables|Default|GetMaxFPS))
  (Variables|/Game/Blueprints/DataContainerObjects/DemoResults.DemoResults_C|SetDuration _asdemoresults_c (- (Variables|Default|GetEndTime) (Variables|Default|GetBeginTime)))
  (SaveGame|SaveGametoSlot _asdemoresults_c (Variables|Default|GetDataSlotName)))

(fn ConstructionScript)

(fn DifferentSecond
  (return (<= 1.0 (- (Utilities|Time|GetGameTimeinSeconds) (Variables|Default|GetLastSecondTime)))))

(fn ChangeSecond
  (if (> (- (Utilities|Time|GetGameTimeinSeconds) (Variables|Default|GetBeginTime)) 1.0)
    ;[1 1 1] Calculate new values
    (Variables|Default|SetLastSecondFPS (Math|Conversions|ToFloat(Integer) (Variables|Default|GetCurrentSecondFrames)))
    (if (> (Variables|Default|GetLastSecondFPS) (Variables|Default|GetMaxFPS))
      (Variables|Default|SetMaxFPS (Variables|Default|GetLastSecondFPS)))
    (if (> (Variables|Default|GetMinFPS) (Variables|Default|GetLastSecondFPS))
      (Variables|Default|SetMinFPS (Variables|Default|GetLastSecondFPS)))
    ;[1 1 1] Reset for next second
    (Variables|Default|SetLastSecondTime (Utilities|Time|GetGameTimeinSeconds))
    (Variables|Default|SetCurrentSecondFrames 0)))