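; PhysicsMetricManager records the results of a physics demo and saves them when play ends.
; On EndPlay it creates a PhysicsResults save object, fills the shared DemoResults data through FillDemoResults, then adds the box count in FillPhysicsResults.
; It writes the object to the DataSlotName save slot and prints an error if saving fails.
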(event EventEndPlay
  (params (EndPlayReason :type EEndPlayReason%20Enum :default "ActorDestroyed"))
  (bind _returnvalue (SaveGame|CreateSaveGameObject "/Game/Blueprints/DataContainerObjects/PhysicsResults.PhysicsResults_C"))
  (bind _asdemoresults_c (Utilities|Casting|CastToDemoResults _returnvalue))
  (CallFunction|FillDemoResults _asdemoresults_c)
  (bind _asphysicsresults_c (Utilities|Casting|CastToPhysicsResults _returnvalue))
  (CallFunction|FillPhysicsResults _asphysicsresults_c)
  (bind _returnvalue_2 (SaveGame|SaveGametoSlot _asphysicsresults_c (Variables|Default|GetDataSlotName)))
  (if (not _returnvalue_2)
    (Development|PrintString "Result Save FAILED")))

(fn ConstructionScript
  (|CallParentFunction))

(fn FillPhysicsResults
  (params (physresults :type Physics%20Results%20Object%20Reference))
  (Variables|/Game/Blueprints/DataContainerObjects/PhysicsResults.PhysicsResults_C|SetBoxCount physresults (Variables|Default|GetBoxCount)))